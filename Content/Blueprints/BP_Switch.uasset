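; BP_Switch is an interactable switch that signals traps of its assigned TrapType through the first-person player character.
; On BeginPlay it caches the player as BP_FirstPersonCharacter and shows the trap type name on its TextRender.
; Interact passes TrapType to the character's CallDPTrap and prints a debug message about turning off the trap, leaving any trap response to be handled outside this Blueprint.
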(event `self.ReceiveBeginPlay`
  (bind _asbp_first_person_character (cast `/Game/Blueprints/Player/BP_FirstPersonCharacter` (`GameplayStatics.GetPlayerCharacter` 0)))
  (set `self.As BP First Person Character` _asbp_first_person_character)
  (`TextRenderComponent.K2_SetText` (`self.TextRender`) (`KismetTextLibrary.Conv_StringToText` (`|GetEnumeratorNameAsString` (`self.TrapType`)))))

(event `/Game/Blueprints/Interface/BPI_Interactable.Interact`
  (`/Game/Blueprints/Player/BP_FirstPersonCharacter.DP_Trap` (`self.As BP First Person Character`) (`self.TrapType`))
  (`KismetSystemLibrary.PrintString` "Turn Of Trap"))

(fn `UserConstructionScript`)