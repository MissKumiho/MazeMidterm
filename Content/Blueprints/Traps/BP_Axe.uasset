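; BP_Axe is a trap that swings an axe and damages the first-person player character.
; Player overlap with a one-shot activation volume enables the damage collider and plays a timeline that pitches the axe group.
; Each player overlap with the damage collider calls DamageUpdate on the character.
; A character-bound trap event with a type check disarms it by destroying the timeline and both colliders.
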(event `self.ReceiveBeginPlay`
  (bind _asbp_first_person_character (cast `/Game/Blueprints/Player/BP_FirstPersonCharacter` (`GameplayStatics.GetPlayerCharacter` 0)))
  (bind _output_get (set `self.As BP First Person Character` _asbp_first_person_character))
  (add `/Game/Blueprints/Player/BP_FirstPersonCharacter.DP_Trap` _output_get (delegate `DP_Trap_Event`)))

(event `DP_Trap_Event`
  (params (TrapType :type "/Game/Blueprints/Enumeration/TrapType Enum" :default "NewEnumerator0"))
  (if (`|EnumEquality` TrapType (`self.TrapType`))
    (`SceneComponent.K2_SetRelativeLocation` (`self.DefaultSceneRoot`) (0.0 0.0 0.0) false false)
    (`PrimitiveComponent.SetCollisionEnabled` (`self.DamageColl`) "NoCollision")
    (`ActorComponent.K2_DestroyComponent` (`self.SpikeMovementTimeline`))
    (`ActorComponent.K2_DestroyComponent` (`self.ActivationColl`))
    (`ActorComponent.K2_DestroyComponent` (`self.DamageColl`))))

(event `self.DamageColl.OnComponentBeginOverlap`
  (params (OverlappedComponent :type "PrimitiveComponent Object Reference") (OtherActor :type "Actor Object Reference") (OtherComp :type "PrimitiveComponent Object Reference") (OtherBodyIndex :type Integer) (bFromSweep :type Boolean) (SweepResult :type "HitResult Structure (by ref)"))
  (if (== OtherActor (`self.As BP First Person Character`))
    (`/Game/Blueprints/Player/BP_FirstPersonCharacter.DamageUpdate` (`self.As BP First Person Character`) 25.0)))

(event `self.ActivationColl.OnComponentBeginOverlap`
  (params (OverlappedComponent :type "PrimitiveComponent Object Reference") (OtherActor :type "Actor Object Reference") (OtherComp :type "PrimitiveComponent Object Reference") (OtherBodyIndex :type Integer) (bFromSweep :type Boolean) (SweepResult :type "HitResult Structure (by ref)"))
  (if (== OtherActor (`self.As BP First Person Character`))
    (`ActorComponent.K2_DestroyComponent` (`self.ActivationColl`))
    (`PrimitiveComponent.SetCollisionEnabled` (`self.DamageColl`) "QueryOnly")
    (bind (_direction _movementtrack) (`Timeline|SpikeMovementTimeline`)
      (:`Update`
        (`SceneComponent.K2_SetRelativeRotation` (`self.AxeGroup`) (`KismetMathLibrary.MakeRotator` 0.0 (`KismetMathLibrary.Lerp` 40.0 -20.0 _movementtrack)) false false)))))

(fn `UserConstructionScript`
  (locals (WallLength :type "Float (double-precision)") (WallThickness :type "Float (double-precision)")))