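; BP_MazeCell is one maze tile that can carry a spike, axe or gas trap and a ceiling light.
; When Ground is set, its construction script scales the floor and adds the flagged walls and ceiling from GridSize and WallHeight, plus a point light if intensity is positive.
; BeginPlay sets the trap's child actor class from TrapType.
; It also binds the player's maze gate dispatcher, recoloring the light to the player's LightColor when IsInside is false.
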(event `self.ReceiveBeginPlay`
  (`|ExecutionSequence`
    (:`then_0`
      (bind _asbp_first_person_character (cast `/Game/Blueprints/Player/BP_FirstPersonCharacter` (`GameplayStatics.GetPlayerCharacter` 0)))
      (bind _output_get (set `self.As BP First Person Character` _asbp_first_person_character))
      (add `/Game/Blueprints/Player/BP_FirstPersonCharacter.DP_Maze_Gate` _output_get (delegate `MazeGate_Event`)))
    (:`then_1`
      (switch `/Game/Blueprints/Enumeration/TrapType` (`self.TrapType`)
        (:`NewEnumerator0`
          (set `self.Trap` false))
        (:`NewEnumerator1`
          (set `self.Trap` true)
          (`ChildActorComponent.SetChildActorClass` (`self.ChildActor`) "/Game/Blueprints/Traps/BP_SpikeTrap.BP_SpikeTrap_C"))
        (:`NewEnumerator2`
          (set `self.Trap` true)
          (`ChildActorComponent.SetChildActorClass` (`self.ChildActor`) "/Game/Blueprints/Traps/BP_Axe.BP_Axe_C"))
        (:`NewEnumerator3`
          (set `self.Trap` true)
          (`ChildActorComponent.SetChildActorClass` (`self.ChildActor`) "/Game/Blueprints/Traps/BP_GasTrap.BP_GasTrap_C"))))))

(event `MazeGate_Event`
  (params (`isInside?` :type Boolean))
  (bind _pointlight (`self.PointLight`))
  (if (not `isInside?`)
    (`/Engine/EditorBlueprintResources/StandardMacros.IsValid` _pointlight
      (:`Is Valid`
        (`KismetSystemLibrary.Delay` 0.1)
        (`LightComponent.SetLightColor` _pointlight (`/Game/Blueprints/Player/BP_FirstPersonCharacter.LightColor` (`self.As BP First Person Character`)) true)))))

(fn `UserConstructionScript`
  (locals (WallLength :type "Float (double-precision)") (WallThickness :type "Float (double-precision)") (NewLocalVar :type "Float (double-precision)"))
  (bind _gridsize (`self.GridSize`))
  (bind _walllength (`local.WallLength`))
  (bind _walllength_2 (`local.WallLength`))
  (bind _returnvalue (* (`local.WallLength`) 0.5))
  (if (`self.Ground`)
    (set `local.WallLength` _gridsize)
    (set `local.WallThickness` (* _gridsize 0.1))
    (`SceneComponent.SetRelativeScale3D` (`self.Floor`) (`self.SizeToCubeScale` (`KismetMathLibrary.MakeVector` _walllength _walllength (`local.WallThickness`))))
    (if (`self.WestWall`)
      (`AddComponent|NODE_AddStaticMeshComponent-0` :`RelativeTransform` (`KismetMathLibrary.MakeTransform` (0.0 0.0 0.0) (struct) (`self.SizeToCubeScale` (`KismetMathLibrary.MakeVector` (`local.WallLength`) (`local.WallThickness`) (`self.WallHeight`))))))
    (if (`self.SouthWall`)
      (`AddComponent|NODE_AddStaticMeshComponent-1` :`RelativeTransform` (`KismetMathLibrary.MakeTransform` (0.0 0.0 0.0) (struct) (`self.SizeToCubeScale` (`KismetMathLibrary.MakeVector` (`local.WallThickness`) (`local.WallLength`) (`self.WallHeight`))))))
    (if (`self.NorthWall`)
      (`AddComponent|NODE_AddStaticMeshComponent-4` :`RelativeTransform` (`KismetMathLibrary.MakeTransform` (`KismetMathLibrary.MakeVector` (- (`local.WallLength`) (`local.WallThickness`))) (struct) (`self.SizeToCubeScale` (`KismetMathLibrary.MakeVector` (`local.WallThickness`) (`local.WallLength`) (`self.WallHeight`))))))
    (if (`self.EastWall`)
      (`AddComponent|NODE_AddStaticMeshComponent-5` :`RelativeTransform` (`KismetMathLibrary.MakeTransform` (`KismetMathLibrary.MakeVector` 0.0 (- (`local.WallLength`) (`local.WallThickness`))) (struct) (`self.SizeToCubeScale` (`KismetMathLibrary.MakeVector` (`local.WallLength`) (`local.WallThickness`) (`self.WallHeight`))))))
    (if (`self.Ceiling`)
      (`AddComponent|NODE_AddStaticMeshComponent-7` :`RelativeTransform` (`KismetMathLibrary.MakeTransform` (`KismetMathLibrary.MakeVector` 0.0 0.0 (`self.WallHeight`)) (struct) (`self.SizeToCubeScale` (`KismetMathLibrary.MakeVector` _walllength_2 _walllength_2 (`local.WallThickness`)))))
      (if (> (`self.LightIntensity`) 0.0)
        (bind _returnvalue_2 (`AddComponent|NODE_AddPointLightComponent-0` :`RelativeTransform` (`KismetMathLibrary.MakeTransform` (`KismetMathLibrary.MakeVector` _returnvalue _returnvalue (* (`self.WallHeight`) 0.9)))))
        (set `self.PointLight` _returnvalue_2)))))